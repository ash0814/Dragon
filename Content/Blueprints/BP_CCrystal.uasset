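; Crystal actor Blueprint that shows its health on a WBP_CrystalHP widget bar.
; BeginPlay caches the widget, and AnyDamage sets its progress bar to CurrentHP / TotalHP without changing the HP values in this graph.
; Tick rotates the widget component toward the player camera so the bar always faces the view.
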(event `self.ReceiveBeginPlay`
  (bind _aswbp_crystal_hp (cast `/Game/UI/WBP_CrystalHP` (`WidgetComponent.GetWidget` (`self.Widget`))))
  (set `self.CrystalHPbar` _aswbp_crystal_hp))

(event `self.ReceiveAnyDamage`
  (params (Damage :type "Float (single-precision)") (DamageType :type "DamageType Object Reference") (InstigatedBy :type "Controller Object Reference") (DamageCauser :type "Actor Object Reference"))
  (set `ProgressBar.Percent` (/ (`self.CurrentHP`) (`self.TotalHP`)) (`/Game/UI/WBP_CrystalHP.ProgressBar_0` (`self.CrystalHPbar`))))

(event `self.ReceiveTick`
  (params (DeltaSeconds :type "Float (single-precision)"))
  (`SceneComponent.K2_SetWorldRotation` (`self.Widget`) (`KismetMathLibrary.FindLookAtRotation` (`SceneComponent.K2_GetComponentLocation` (`self.Widget`)) (`SceneComponent.K2_GetComponentLocation` (`PlayerCameraManager.TransformComponent` (`GameplayStatics.GetPlayerCameraManager` 0)))) false false))

(fn `UserConstructionScript`)